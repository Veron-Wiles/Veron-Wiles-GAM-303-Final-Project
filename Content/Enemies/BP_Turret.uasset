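; BP_Turret is an enemy turret that tracks and shoots the player while they are inside its Box trigger.
; Player overlap starts two looping function-name timers, one for aiming and one for firing, and leaving the box clears both.
; Aiming rotates the Pivot toward the player with pitch held at zero, and firing spawns a BP_TurretBullet at the BulletSpawn transform.
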(event `FireAtPlayer`
  ; Shoot at Player
  (`|SpawnActorFromClass` "/Game/Enemies/BP_TurretBullet.BP_TurretBullet_C" (`SceneComponent.K2_GetComponentToWorld` (`self.BulletSpawn`)) "Undefined" "MultiplyWithRoot" null null))

(event `FollowPlayer`
  (bind (_returnvalue_roll _returnvalue_pitch _returnvalue_yaw) (`KismetMathLibrary.BreakRotator` (`KismetMathLibrary.FindLookAtRotation` (`self.K2_GetActorLocation`) (`self.K2_GetActorLocation` (`GameplayStatics.GetPlayerCharacter` 0)))))
  ; Follow The Player
  (`SceneComponent.K2_SetWorldRotation` (`self.Pivot`) (`KismetMathLibrary.MakeRotator` _returnvalue_roll 0.0 _returnvalue_yaw) false false))

(event `self.Box.OnComponentBeginOverlap`
  (params (OverlappedComponent :type "PrimitiveComponent Object Reference") (OtherActor :type "Actor Object Reference") (OtherComp :type "PrimitiveComponent Object Reference") (OtherBodyIndex :type Integer) (bFromSweep :type Boolean) (SweepResult :type "HitResult Structure (by ref)"))
  ; Start timers if player enters
  (cast `/Game/Player/BP_Player` OtherActor)
  (`KismetSystemLibrary.K2_SetTimer` null "FollowPlayer" 0.05 true)
  (`KismetSystemLibrary.K2_SetTimer` null "FireAtPlayer" 0.5 true))

(event `self.Box.OnComponentEndOverlap`
  (params (OverlappedComponent :type "PrimitiveComponent Object Reference") (OtherActor :type "Actor Object Reference") (OtherComp :type "PrimitiveComponent Object Reference") (OtherBodyIndex :type Integer))
  ; Clear timers if player leaves
  (cast `/Game/Player/BP_Player` OtherActor)
  (`KismetSystemLibrary.K2_ClearTimer` null "FollowPlayer")
  (`KismetSystemLibrary.K2_ClearTimer` null "FireAtPlayer"))

(fn `UserConstructionScript`)