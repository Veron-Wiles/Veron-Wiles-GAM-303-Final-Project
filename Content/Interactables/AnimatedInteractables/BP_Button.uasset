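; BP_Button is a color-coded pressure button that unlocks its TargetDoor while a BP_Gun of matching PickupColor rests in its overlap volume.
; A match sets IsUnlocked on the door and plays a timeline that lowers the button mesh, printing a message instead if no door is set.
; Any BP_Gun leaving relocks the door and reverses the timeline, without a color check.
; The construction script tints the mesh to ButtonColor through a dynamic material.
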(event `self.Overlap.OnComponentBeginOverlap`
  (params (OverlappedComponent :type "PrimitiveComponent Object Reference") (OtherActor :type "Actor Object Reference") (OtherComp :type "PrimitiveComponent Object Reference") (OtherBodyIndex :type Integer) (bFromSweep :type Boolean) (SweepResult :type "HitResult Structure (by ref)"))
  (bind _targetdoor (`self.TargetDoor`))
  ; Press Button with Object
  (bind _asbp_gun (cast `/Game/Interactables/BP_Gun` OtherActor))
  (if (== (`/Game/Interactables/BP_Gun.Pickup Color` _asbp_gun) (`self.Button Color`))
    (`/Engine/EditorBlueprintResources/StandardMacros.IsValid` _targetdoor
      (:`Is Valid`
        (set `/Game/Interactables/AnimatedInteractables/BP_Door.IsUnlocked` true _targetdoor)
        (bind (_direction _alphatrack) (`Timeline|Alpha` :!label _label)
          (:`Update`
            (`SceneComponent.K2_SetRelativeLocation` (`self.Button`) (`KismetMathLibrary.MakeVector` 0.0 0.0 (`KismetMathLibrary.Lerp` 5.0 1.0 _alphatrack)) false false))))
      (:`Is Not Valid`
        (`KismetSystemLibrary.PrintString` "No Door set")))))

(event `self.Overlap.OnComponentEndOverlap`
  (params (OverlappedComponent :type "PrimitiveComponent Object Reference") (OtherActor :type "Actor Object Reference") (OtherComp :type "PrimitiveComponent Object Reference") (OtherBodyIndex :type Integer))
  ; Press Button with Object
  (cast `/Game/Interactables/BP_Gun` OtherActor)
  (set `/Game/Interactables/AnimatedInteractables/BP_Door.IsUnlocked` false (`self.TargetDoor`))
  (goto _label :!via `Reverse`))

(fn `UserConstructionScript`
  (bind _returnvalue (`PrimitiveComponent.CreateDynamicMaterialInstance` (`self.Button`) 0 "/Game/Materials/MAT_Color.MAT_Color" "None"))
  (bind _output_get (set `self.Color DMI` _returnvalue))
  (`MaterialInstanceDynamic.SetVectorParameterValue` _output_get "Color" (`self.Button Color`)))