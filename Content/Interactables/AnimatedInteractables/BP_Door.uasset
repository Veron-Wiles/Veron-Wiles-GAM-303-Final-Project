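; BP_Door is an interactable door that swings open when a player interacts with it, then closes itself.
; A dot product of the direction to the player and the door's forward vector picks a positive or negative quarter-turn swing, based on the player's side.
; A Timeline drives the yaw of an Arrow component as the pivot, then reverses after a short delay once fully open.
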(event `/Game/Interfaces/INT_Interact.INT_Interact`
  (params (Player :type "/Game/Player/BP_Player Object Reference"))
  ; Open Door on Interact
  (bind _returnvalue (`self.NewFunction` Player))
  (bind (_direction _alpha) (`Timeline|Timeline` :!via `PlayFromStart` :!label _label)
    (:`Update`
      (`SceneComponent.K2_SetRelativeRotation` (`self.Arrow`) (`KismetMathLibrary.MakeRotator` 0.0 0.0 (`KismetMathLibrary.Lerp` 0.0 _returnvalue _alpha)) false false))
    (:`Finished`
      (if (`|EnumEquality` _direction "Forward")
        (`KismetSystemLibrary.Delay` 0.2)
        (`self.CloseDoor`)))))

(event `CloseDoor`
  ; Open Door on Interact
  (goto _label :!via `ReverseFromEnd`))

(fn `NewFunction`
  (params (self2 :type "Actor Object Reference"))
  (returns (ReturnValue :type "Float (double-precision)"))
  (return (select `bool` (> (`KismetMathLibrary.Dot_VectorVector` (`KismetMathLibrary.GetDirectionUnitVector` (`self.K2_GetActorLocation`) (`self.K2_GetActorLocation` self2)) (`self.GetActorForwardVector`)) 0.0) :`false` -90.0 :`true` 90.0)))

(fn `UserConstructionScript`)