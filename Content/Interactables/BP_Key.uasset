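; BP_Key is a colored key item that the player can pick up and drop through grab and drop interface events.
; Grabbing, allowed only with an empty hand, flags the player as holding an item, disables the cube's physics and collision, and snaps it to the holding hand.
; Dropping detaches it and restores collision and physics, without clearing the holding flag here.
; The construction script tints the cube with KeyColor through a dynamic material instance.
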(event `/Game/Interfaces/INT_Interact.INT_Grab`
  (params (Player :type "/Game/Player/BP_Player Object Reference"))
  (bind _cube (`self.Cube`))
  ; Pick Up
  (if (not (`/Game/Player/BP_Player.IsHoldingItem` Player))
    (set `/Game/Player/BP_Player.IsHoldingItem` true Player)
    (`PrimitiveComponent.SetSimulatePhysics` _cube false)
    (`PrimitiveComponent.SetCollisionEnabled` _cube "NoCollision")
    (`SceneComponent.K2_AttachToComponent` _cube (`/Game/Player/BP_Player.HoldingHand` Player) "None" "SnapToTarget" "SnapToTarget" "KeepRelative" true)))

(event `/Game/Interfaces/INT_Interact.INT_Drop`
  (bind _cube (`self.Cube`))
  ; Drop
  (`self.K2_DetachFromActor` "KeepWorld" "KeepWorld" "KeepWorld")
  (`PrimitiveComponent.SetCollisionEnabled` _cube "QueryAndPhysics")
  (`PrimitiveComponent.SetSimulatePhysics` _cube true))

(fn `UserConstructionScript`
  (bind _returnvalue (`PrimitiveComponent.CreateDynamicMaterialInstance` (`self.Cube`) 0 "/Game/Materials/MAT_Color.MAT_Color" "None"))
  (bind _output_get (set `self.Color DMI` _returnvalue))
  (`MaterialInstanceDynamic.SetVectorParameterValue` _output_get "Color" (`self.Key Color`)))