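; BP_Player is the player pawn, handling Enhanced Input movement, yaw-only look, object interaction and health gain.
; Interact line-traces from the camera, sending a grab message to physics-simulating hits when not holding, and an interact message to non-simulating hits.
; Drop messages the held object and clears the holding flag, which this graph never sets true.
; AddHealth applies and prints gains only when they stay within maximum health.
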(event `DropItem`
  ; Drop Item
  (message `/Game/Interfaces/INT_Interact.INT_Drop` (`self.HeldObject`))
  (set `self.IsHolding` false))

(event `Interact`
  (bind _camera (`self.Camera`))
  (bind _returnvalue (`SceneComponent.K2_GetComponentLocation` _camera))
  ; Interact with Interactable
  (bind (_outhit _returnvalue_2) (`KismetSystemLibrary.LineTraceSingle` :`Start` _returnvalue :`End` (+ _returnvalue (* (`SceneComponent.GetForwardVector` _camera) (800.0 800.0 800.0))) :`TraceChannel` "TraceTypeQuery1" :`DrawDebugType` "ForDuration"))
  (if _returnvalue_2
    (bind (_bblockinghit _binitialoverlap _time _distance _location _impactpoint _normal _impactnormal _physmat _hitactor _hitcomponent) (`GameplayStatics.BreakHitResult` _outhit))
    (if (`SceneComponent.IsSimulatingPhysics` _hitcomponent "None")
      (if (not (`self.IsHolding`))
        (set `self.HeldObject` _hitactor)
        (message `/Game/Interfaces/INT_Interact.INT_Grab` _hitactor self))
      (else
        (message `/Game/Interfaces/INT_Interact.INT_Interact` _hitactor self)))))

(event `AddHealth`
  (params (B :type Integer))
  (bind _returnvalue (+ (`self.CurrentHealth`) B))
  ; Add Health
  (if (<= _returnvalue (`self.MaxHealth`))
    (bind _output_get (set `self.CurrentHealth` _returnvalue))
    (`KismetSystemLibrary.PrintString` (`KismetStringLibrary.Conv_IntToString` _output_get))))

(event `EnhancedInput|/Game/Player/IA_PlayerDrop`
  (params (ActionValue :type Boolean) (ElapsedSeconds :type "Float (double-precision)") (TriggeredSeconds :type "Float (double-precision)") (InputAction :type "InputAction Object Reference" :default "/Game/Player/IA_PlayerDrop.IA_PlayerDrop"))
  ; Check for Drop Button
  (:`Triggered`
    (if (`self.IsHolding`)
      (`self.DropItem`))))

(event `EnhancedInput|/Game/Player/IA_PlayerInteract`
  (params (ActionValue :type Boolean) (ElapsedSeconds :type "Float (double-precision)") (TriggeredSeconds :type "Float (double-precision)") (InputAction :type "InputAction Object Reference" :default "/Game/Player/IA_PlayerInteract.IA_PlayerInteract"))
  ; Check for Interact Button
  (:`Triggered`
    (`self.Interact`)))

(event `EnhancedInput|/Game/Player/IA_PlayerLook`
  (params (ActionValue :type "Float (double-precision)") (ElapsedSeconds :type "Float (double-precision)") (TriggeredSeconds :type "Float (double-precision)") (InputAction :type "InputAction Object Reference" :default "/Game/Player/IA_PlayerLook.IA_PlayerLook"))
  ; Turn Player
  (:`Triggered`
    (`self.AddControllerYawInput` ActionValue)))

(event `EnhancedInput|/Game/Player/IA_PlayerMove`
  (params (ActionValue :type "Vector2D Structure") (ElapsedSeconds :type "Float (double-precision)") (TriggeredSeconds :type "Float (double-precision)") (InputAction :type "InputAction Object Reference" :default "/Game/Player/IA_PlayerMove.IA_PlayerMove"))
  (bind _capsulecomponent (`self.CapsuleComponent`))
  ; Move Player
  (:`Triggered`
    (`self.AddMovementInput` (`SceneComponent.GetForwardVector` _capsulecomponent) ActionValue_Y)
    (`self.AddMovementInput` (`SceneComponent.GetRightVector` _capsulecomponent) ActionValue_X)))

(fn `UserConstructionScript`)